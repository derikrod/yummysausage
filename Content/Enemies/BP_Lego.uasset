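; BP_Lego is an enemy-folder hazard that knocks the player's sausage character away on hit.
; BeginPlay caches the BP_sausage pawn and sets the timeline's play rate from PlayRate.
; The timeline's update lerps the Lego component's pitch to swing it, though nothing in the graph starts it.
; Any Hit launches the cached sausage along the Lego's normalized velocity at fixed strength, without checking what was hit.
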(event EventBeginPlay
  (bind _asbp_sausage (Utilities|Casting|CastToBP_sausage (Game|Player|GetPlayerPawn 0)))
  (Variables|Default|SetSausage_refer _asbp_sausage)
  (Components|Timeline|SetPlayRate (Variables|Default|GetTimeline_0) (Variables|Default|GetPlayRate)))

(event Collision|EventActorBeginOverlap
  (params (OtherActor :type Actor%20Object%20Reference)))

(event EventTick
  (params (DeltaSeconds :type Float%20%28single-precision%29)))

(event Collision|EventHit
  (params (MyComp :type Primitive%20Component%20Object%20Reference) (Other :type Actor%20Object%20Reference) (OtherComp :type Primitive%20Component%20Object%20Reference) (bSelfMoved :type Boolean) (HitLocation :type Vector :default "0, 0, 0") (HitNormal :type Vector :default "0, 0, 0") (NormalImpulse :type Vector :default "0, 0, 0") (Hit :type Hit%20Result%20Structure%20%28by%20ref%29))
  (Character|LaunchCharacter (Variables|Default|GetSausage_refer) (* (Math|Vector|Normalize (Transformation|GetComponentVelocity (Variables|Default|Getlego))) 2e+03) false false))

(fn ConstructionScript)