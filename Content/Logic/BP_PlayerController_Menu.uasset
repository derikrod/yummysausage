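; Menu player controller that runs the main menu, how-to-play and loading screen widgets.
; It creates all three on BeginPlay and shows the main menu.
; A shared CallHudMenu event adds or removes the selected widget and sets input mode and cursor visibility.
; Game start swaps to the loading screen, centers the mouse, waits briefly, then sends a map-change message to the first actor implementing BPI_GameInstance.
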(event EventBeginPlay
  (bind _returnvalue (Game|GetPlayerController 0))
  ;[0.4869 1 0.2746] UI
  ;;[1 1 1] Control Hud Based on Map
  (Utilities|FlowControl|Sequence
    (:then_0
      (bind _returnvalue_2 (UserInterface|CreateWidget "/Game/Logic/HUD/WBP_mainMenu.WBP_mainMenu_C" _returnvalue))
      (Variables|Default|SetMainMenuReffer _returnvalue_2)
      (CallFunction|CallHudMenu true "NewEnumerator0" "NewEnumerator2" true))
    (:then_1
      (bind _returnvalue_3 (UserInterface|CreateWidget "/Game/Logic/HUD/WBP_howtoplay.WBP_howtoplay_C" _returnvalue))
      (Variables|Default|SethowtoPlayReffer _returnvalue_3))
    (:then_2
      (bind _returnvalue_4 (UserInterface|CreateWidget "/Game/Logic/HUD/WPB_loading.WPB_loading_C" _returnvalue))
      (Variables|Default|SetLoadingReffer _returnvalue_4))))

(event EventTick
  (params (DeltaSeconds :type Float%20%28single-precision%29)))

(event EventCallHudMenu
  (params (Show :type Boolean) (Menu :type E_huds_menu%20Enum :default "NewEnumerator0") (InputType :type E_inputTypes%20Enum :default "NewEnumerator0") (ShowMouse :type Boolean))
  (bind _returnvalue (Game|GetPlayerController 0))
  (bind _mainmenureffer (Variables|Default|GetMainMenuReffer))
  (bind _howtoplayreffer (Variables|Default|GethowtoPlayReffer))
  (bind _loadingreffer (Variables|Default|GetLoadingReffer))
  (bind _returnvalue_2 (Utilities|Select :Index Menu :NewEnumerator0 _mainmenureffer :NewEnumerator1 _loadingreffer :NewEnumerator2 _howtoplayreffer))
  ;[0.4869 1 0.2746] UI
  ;;[1 1 1] Call menus show/hide
  (bind _output_get (Variables|Default|SetShow Show))
  (if _output_get
    (UserInterface|Viewport|AddtoViewport _returnvalue_2 0)
    (else
      (Widget|RemovefromParent _returnvalue_2)))
  (switch Utilities|FlowControl|Switch|SwitchonE_inputTypes InputType
    (:NewEnumerator0
      (Input|SetInputModeGameOnly _returnvalue))
    (:NewEnumerator1
      (Input|SetInputModeUIOnly _returnvalue 0 "DoNotLock"))
    (:NewEnumerator2
      (Input|SetInputModeGameandUI _returnvalue 0 "DoNotLock" true)))
  (Variables|/Script/Engine.PlayerController|SetbShowMouseCursor _returnvalue ShowMouse))

(event EventShowHowtoplay
  ;[0.4869 1 0.2746] UI
  ;;[1 1 1] MainMenuButtons Interactions
  (CallFunction|CallHudMenu true "NewEnumerator2" "NewEnumerator1" true))

(event EventCloseHowtoPlay
  ;[0.4869 1 0.2746] UI
  ;;[1 1 1] MainMenuButtons Interactions
  (CallFunction|CallHudMenu false "NewEnumerator2" "NewEnumerator1" true))

(event EventCallGameStart
  (bind _returnvalue (Game|GetPlayerController 0))
  (bind (_sizex _sizey) (HUD|GetViewportSize _returnvalue))
  ;[0.4869 1 0.2746] UI
  ;;[1 1 1] MainMenuButtons Interactions
  (CallFunction|CallHudMenu false "NewEnumerator0" "NewEnumerator0" false)
  (CallFunction|CallHudMenu true "NewEnumerator1" "NewEnumerator0" false)
  (Class|PlayerController|SetMouseLocation _returnvalue (/ _sizex 2) (/ _sizey 2))
  (Utilities|FlowControl|Delay 2.0)
  (bind _outactors (Actor|GetAllActorswithInterface "/Game/Logic/BPI_GameInstance.BPI_GameInstance_C"))
  (Class|BPIGameInstance|ChangeMap(Message) (Utilities|Array|Get(acopy) _outactors) "NewEnumerator1"))

(fn ConstructionScript)