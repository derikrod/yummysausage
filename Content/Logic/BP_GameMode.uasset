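; Game mode Blueprint that handles level flow: restarting, quitting to the Main level and changing maps.
; Restart runs the RestartLevel console command, while ChangeMap maps an enum value to a level name and opens it.
; GetMap always returns MainMenu.
; The spice mode sound events are empty, and their music fade, scream and sound-spawn nodes are left disconnected and never run.
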(event Custom|Restart
  ;[1 1 1] Spice Mode Sound
  (Development|ExecuteConsoleCommand "RestartLevel" 0))

(event Custom|Quit
  ;[1 1 1] Spice Mode Sound
  (Game|OpenLevel(byName) "Main"))

(event Custom|PlaySpiceSound
  ;[1 1 1] Spice Mode Sound
)

(event Custom|FinishSpiceSound
  ;[1 1 1] Spice Mode Sound
)

(event EventBeginPlay)

(event EventChangeMap
  (params (Map :type E_Maps%20Enum :default "NewEnumerator0"))
  (Game|OpenLevel(byName) (Utilities|Select :Index Map :NewEnumerator0 "Main" :NewEnumerator1 "Map1")))

(fn ConstructionScript)

(fn GetMap
  (return "NewEnumerator0"))