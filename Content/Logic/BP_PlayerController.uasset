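; Player controller that owns the game's UI: the life bar, pause and end-result widgets, all created at BeginPlay.
; A shared CallMenu event adds or removes the selected widget and sets input mode and cursor visibility.
; The pause input alternates pause and unpause via FlipFlop, passing SetGamePaused's return value as the menu's show flag.
; It binds to the first BP_hotdog's game-end event to show the final intoxication result on the end screen.
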(event Custom|ShowResult
  (params (finalIntoxication :type Float%20%28single-precision%29))
  ;[0.4869 1 0.2746] UI
  ;;[1 1 1] Control Hud Based on Map
  (Default|GetFinalResult (Variables|Default|GetEndReffer) finalIntoxication)
  (CallFunction|CallMenu true "NewEnumerator5" "NewEnumerator1" true))

(event Custom|PauseGame
  ;[0.4869 1 0.2746] UI
  (bind _returnvalue (Game|SetGamePaused true))
  (CallFunction|CallMenu _returnvalue "NewEnumerator4" "NewEnumerator0" true))

(event Custom|UnpauseGame
  ;[0.4869 1 0.2746] UI
  (bind _returnvalue (Game|SetGamePaused false))
  (CallFunction|CallMenu _returnvalue "NewEnumerator4" "NewEnumerator0" true))

(event EventBeginPlay
  (bind _returnvalue (Game|GetPlayerController 0))
  ;[0.4869 1 0.2746] UI
  ;;[1 1 1] Control Hud Based on Map
  (Utilities|FlowControl|Sequence
    (:then_0
      (bind _returnvalue_2 (UserInterface|CreateWidget "/Game/Logic/HUD/WBP_life.WBP_life_C" _returnvalue))
      (Variables|Default|SetLifebarReffer _returnvalue_2)
      (CallFunction|CallMenu true "NewEnumerator3" "NewEnumerator0" false))
    (:then_1
      (bind _returnvalue_3 (UserInterface|CreateWidget "/Game/Logic/HUD/WBP_pause.WBP_pause_C" _returnvalue))
      (Variables|Default|SetPauseReffer _returnvalue_3))
    (:then_2
      (bind _returnvalue_4 (UserInterface|CreateWidget "/Game/Logic/HUD/WBP_end.WBP_end_C" _returnvalue))
      (Variables|Default|SetEndReffer _returnvalue_4))
    (:then_3
      (bind _outactors (Actor|GetAllActorsOfClass "/Game/Evironment/BP_hotdog.BP_hotdog_C"))
      (bind _output_get (Variables|Default|SethotDogReffer (Utilities|Array|Get(acopy) _outactors)))
      (EventDispatchers|BindEventtoGameIsend _output_get (delegate Custom|ShowResult)))))

(event EventTick
  (params (DeltaSeconds :type Float%20%28single-precision%29)))

(event EventCallMenu
  (params (Show :type Boolean) (Menu :type E_huds%20Enum :default "NewEnumerator3") (InputType :type E_inputTypes%20Enum :default "NewEnumerator0") (ShowMouse :type Boolean))
  (bind _returnvalue (Game|GetPlayerController 0))
  (bind _endreffer (Variables|Default|GetEndReffer))
  (bind _pausereffer (Variables|Default|GetPauseReffer))
  (bind _lifebarreffer (Variables|Default|GetLifebarReffer))
  (bind _returnvalue_2 (Utilities|Select :Index Menu :NewEnumerator3 _lifebarreffer :NewEnumerator4 _pausereffer :NewEnumerator5 _endreffer))
  ;[0.4869 1 0.2746] UI
  ;;[1 1 1] Call menus show/hide
  (bind _output_get (Variables|Default|SetShow Show))
  (if _output_get
    (UserInterface|Viewport|AddtoViewport _returnvalue_2 0)
    (else
      (Widget|RemovefromParent _returnvalue_2)))
  (switch Utilities|FlowControl|Switch|SwitchonE_inputTypes InputType
    (:NewEnumerator0
      (Input|SetInputModeGameOnly _returnvalue))
    (:NewEnumerator1
      (Input|SetInputModeUIOnly _returnvalue _returnvalue_2 "DoNotLock"))
    (:NewEnumerator2
      (Input|SetInputModeGameandUI _returnvalue _returnvalue_2 "DoNotLock" true)))
  (Variables|/Script/Engine.PlayerController|SetbShowMouseCursor _returnvalue ShowMouse))

(event Input|ActionEvents|InputActionPauseButtom
  (params (Key :type Key%20Structure :default "None"))
  ;[0.4869 1 0.2746] UI
  (:Pressed
    (Utilities|FlowControl|FlipFlop
      (:A
        (CallFunction|PauseGame))
      (:B
        (CallFunction|UnpauseGame)))))

(fn ConstructionScript)