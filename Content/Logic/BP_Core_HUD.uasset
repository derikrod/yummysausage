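; BP_Core_HUD is a HUD manager that shows and hides the game's main menu, loading, how-to-play, life bar, pause and end screens.
; The Callhud event switches on a HUD type and adds or removes the matching stored widget from the viewport, while CallhudReffer returns that widget reference by type.
; Widget creation nodes for all but the main menu are present but disconnected, so this graph never fills those references.
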(event EventCallhud
  (params (Hudtype :type E_huds%20Enum :default "NewEnumerator0") (Show :type Boolean))
  (bind _mainmenureffer (Variables|Default|GetMainMenuReffer))
  (bind _loadingreffer (Variables|Default|GetLoadingReffer))
  (bind _howtoplayreffer (Variables|Default|GetHowtoPlayReffer))
  (bind _lifebarreffer (Variables|Default|GetLifebarReffer))
  (bind _pausereffer (Variables|Default|GetPauseReffer))
  (bind _endreffer (Variables|Default|GetEndReffer))
  (Variables|Default|SetShow Show)
  (switch Utilities|FlowControl|Switch|SwitchonE_huds Hudtype
    (:NewEnumerator0
      (if (Variables|Default|GetShow)
        (UserInterface|Viewport|AddtoViewport _mainmenureffer 0)
        (else
          (Widget|RemovefromParent _mainmenureffer))))
    (:NewEnumerator1
      (if (Variables|Default|GetShow)
        (UserInterface|Viewport|AddtoViewport _loadingreffer 0)
        (else
          (Widget|RemovefromParent _loadingreffer))))
    (:NewEnumerator2
      (if (Variables|Default|GetShow)
        (UserInterface|Viewport|AddtoViewport _howtoplayreffer 0)
        (else
          (Widget|RemovefromParent _howtoplayreffer))))
    (:NewEnumerator3
      (if (Variables|Default|GetShow)
        (UserInterface|Viewport|AddtoViewport _lifebarreffer 0)
        (else
          (Widget|RemovefromParent _lifebarreffer))))
    (:NewEnumerator4
      (if (Variables|Default|GetShow)
        (UserInterface|Viewport|AddtoViewport _pausereffer 0)
        (else
          (Widget|RemovefromParent _pausereffer))))
    (:NewEnumerator5
      (if (Variables|Default|GetShow)
        (UserInterface|Viewport|AddtoViewport _endreffer 0)
        (else
          (Widget|RemovefromParent _endreffer))))))

(fn ConstructionScript)

(fn CallhudReffer
  (params (HudType :type E_huds%20Enum :default "NewEnumerator0"))
  (return (Utilities|Select :Index HudType :NewEnumerator0 (Variables|Default|GetMainMenuReffer) :NewEnumerator1 (Variables|Default|GetLoadingReffer) :NewEnumerator2 (Variables|Default|GetHowtoPlayReffer) :NewEnumerator3 (Variables|Default|GetLifebarReffer) :NewEnumerator4 (Variables|Default|GetPauseReffer) :NewEnumerator5 (Variables|Default|GetEndReffer))))