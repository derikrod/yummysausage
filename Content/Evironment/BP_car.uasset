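; Car actor that plays a one-time cutscene of its mesh travelling along a spline when first overlapped by any actor.
; The overlap blends the player's view to this actor and blocks move and look input, then starts a timeline after a short delay.
; The timeline moves the mesh along the spline, mapping negated spline pitch to roll with fixed yaw.
; When it finishes, view and input return to the player character.
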(event EventBeginPlay
  (bind _asbp_sausage (Utilities|Casting|CastToBP_sausage (Game|Player|GetPlayerPawn 0)))
  (Variables|Default|SetSausageReffer _asbp_sausage))

(event Collision|EventActorBeginOverlap
  (params (OtherActor :type Actor%20Object%20Reference))
  (bind _spline (Variables|Default|GetSpline))
  (Utilities|FlowControl|DoOnce false
    (:Completed
      (CallFunction|OpenCamera)
      (Utilities|FlowControl|Delay 2.0)
      (bind _newtrack_0 (Timeline|PathTimeline Play)
        (:Update
          (Utilities|FlowControl|Sequence
            (:then_0
              (Transformation|SetWorldLocation (Variables|Default|GetStaticMesh) (Spline|GetLocationatDistanceAlongSpline _spline (* _newtrack_0 (Spline|GetSplineLength _spline)) "World") false false))
            (:then_1
              (Transformation|SetRelativeRotation (Variables|Default|GetStaticMesh) (Math|Rotator|MakeRotator (* (.pitch (Spline|GetRotationatDistanceAlongSpline _spline (* _newtrack_0 (Spline|GetSplineLength _spline)) "World")) -1.0) 0.0 -9e+01) false false))))
        (:Finished
          (CallFunction|CloseCamera))))))

(event EventTick
  (params (DeltaSeconds :type Float%20%28single-precision%29)))

(fn ConstructionScript)

(fn OpenCamera
  (bind _returnvalue (Game|GetPlayerController 0))
  (Game|Player|SetViewTargetwithBlend _returnvalue self 2.0 "VTBlend_Linear" 0.0 false)
  (Input|SetIgnoreMoveInput _returnvalue true)
  (Input|SetIgnoreLookInput _returnvalue true))

(fn CloseCamera
  (bind _returnvalue (Game|GetPlayerController 0))
  (Game|Player|SetViewTargetwithBlend _returnvalue (Game|GetPlayerCharacter 0) 0.0 "VTBlend_Linear" 0.0 false)
  (Input|ResetIgnoreMoveInput _returnvalue)
  (Input|ResetIgnoreLookInput _returnvalue))