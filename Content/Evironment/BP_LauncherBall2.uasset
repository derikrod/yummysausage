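; BP_LauncherBall2 is a bouncy ball that launches the player's BP_sausage upward when it registers a hit.
; Each hit restarts a timeline that drives the Ball's "squash" morph target.
; After a short delay, a DoOnce launches the sausage and plays a jump sound, then stays closed until the timeline finishes.
; The launch always targets the player pawn cached at BeginPlay, without checking what hit the ball.
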(event EventBeginPlay
  (bind _asbp_sausage (Utilities|Casting|CastToBP_sausage (Game|Player|GetPlayerPawn 0)))
  (Variables|Default|SetSausage_reffer _asbp_sausage))

(event EventTick
  (params (DeltaSeconds :type Float%20%28single-precision%29)))

(event Collision|EventHit
  (params (MyComp :type Primitive%20Component%20Object%20Reference) (Other :type Actor%20Object%20Reference) (OtherComp :type Primitive%20Component%20Object%20Reference) (bSelfMoved :type Boolean) (HitLocation :type Vector :default "0, 0, 0") (HitNormal :type Vector :default "0, 0, 0") (NormalImpulse :type Vector :default "0, 0, 0") (Hit :type Hit%20Result%20Structure%20%28by%20ref%29))
  (Utilities|FlowControl|Sequence
    (:then_0
      (bind _newtrack_0 (Timeline|Timeline_0 PlayFromStart)
        (:Update
          (Components|SkeletalMesh|SetMorphTarget (Variables|Default|Getball) "squash" _newtrack_0 true))
        (:Finished
          (goto _label Reset))))
    (:then_1
      (Utilities|FlowControl|Delay 0.2)
      (Utilities|FlowControl|DoOnce false :!label _label
        (:Completed
          (Character|LaunchCharacter (Variables|Default|GetSausage_reffer) "0, 0,1000.000000" false false)
          (Audio|PlaySoundatLocation "/Game/sounds/balljump.balljump" (Transformation|GetActorLocation) "0, 0, 0" 1.0 1.0 0.0 0 0 0))))))

(fn ConstructionScript)