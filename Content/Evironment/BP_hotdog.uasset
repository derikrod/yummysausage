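; BP_hotdog is the level's end goal, a spinning hotdog that takes in the player's sausage and ends the game.
; On any overlap it hides the player mesh and reveals its own sausage, copying flatness and putrefaction-blended color into a dynamic material.
; It then stops rotating, blends the camera to itself and swaps its Niagara effect for a bright burst.
; After a short delay it calls GameIsend with the sausage's Life.
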(event EventBeginPlay
  (Utilities|FlowControl|Sequence
    (:then_0
      (bind _asbp_sausage (Utilities|Casting|CastToBP_sausage (Game|Player|GetPlayerPawn 0)))
      (Variables|Default|SetSausage_reffer _asbp_sausage))
    (:then_1
      (bind _asbp_game_mode (Utilities|Casting|CastToBP_GameMode (Game|GetGameMode)))
      (Variables|Default|SetAs%20BP%20Game%20Mode _asbp_game_mode))))

(event Collision|EventActorBeginOverlap
  (params (OtherActor :type Actor%20Object%20Reference))
  (bind _sausage_reffer (Variables|Default|GetSausage_reffer))
  (Rendering|SetVisibility (Variables|/Script/Engine.Character|GetMesh (Variables|Default|GetSausage_reffer)) false false)
  (Rendering|Material|SetScalarParameterValue (Variables|Default|GetsausageMesh) "Flatness" (Variables|/Game/Character/BP_sausage.BP_sausage_C|Getflatness (Variables|Default|GetSausage_reffer)) :!class /Script/Engine.MaterialInstanceDynamic)
  (Rendering|Material|SetVectorParameterValue (Variables|Default|GetsausageMesh) "BaseColor" (Math|Conversions|ToLinearColor(Vector) (Math|Vector|Lerp(Vector) (Math|Conversions|ToVector(LinearColor) (Variables|/Game/Character/BP_sausage.BP_sausage_C|GetBaseolor _sausage_reffer)) (Math|Conversions|ToVector(LinearColor) (Variables|/Game/Character/BP_sausage.BP_sausage_C|GetNewcolor _sausage_reffer)) (Variables|/Game/Character/BP_sausage.BP_sausage_C|Getputrification _sausage_reffer))) :!class /Script/Engine.MaterialInstanceDynamic)
  (Rendering|SetVisibility (Variables|Default|Gethotdog_sausage) true false)
  (Variables|/Script/Engine.RotatingMovementComponent|SetRotationRate (Variables|Default|GetRotatingMovement) "0, 0, 0")
  (Transformation|SetActorRelativeRotation "0, 0, 0")
  (Game|Player|SetViewTargetwithBlend (Game|GetPlayerController 0) self 0.5 "VTBlend_Linear" 0.0 false)
  (Rendering|SetVisibility (Variables|Default|GetNiagara) false false)
  (Niagara|SpawnSystematLocation "/Game/FX/NS_Brightburst.NS_Brightburst" (Transformation|GetActorLocation))
  (Utilities|FlowControl|Delay 0.7)
  (Default|CallGameIsend (Variables|/Game/Character/BP_sausage.BP_sausage_C|Getlife (Variables|Default|GetSausage_reffer))))

(event EventTick
  (params (DeltaSeconds :type Float%20%28single-precision%29)))

(fn ConstructionScript
  (bind _returnvalue (Rendering|Material|CreateDynamicMaterialInstance (Variables|Default|Gethotdog_sausage) 0 "/Game/Character/FBX/M_sausage_Emissive.M_sausage_Emissive" "None" :!class /Script/Engine.PrimitiveComponent))
  (Variables|Default|SetsausageMesh _returnvalue))