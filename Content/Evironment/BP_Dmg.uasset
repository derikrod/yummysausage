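; BP_Dmg is an environment hazard actor, apparently a floor, that raises the player sausage's Damage value while something overlaps it.
; BeginPlay caches the player pawn as BP_sausage, and overlap events act on that reference without checking the overlapping actor.
; Overlap flags it as on floor and, unless hot, raises Damage and shows a warning, escalating after a delay if still flagged.
; Ending overlap resets both and hides the message.
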(event EventBeginPlay
  (Utilities|FlowControl|Sequence
    (:then_0
      (bind _asbp_sausage (Utilities|Casting|CastToBP_sausage (Game|Player|GetPlayerPawn 0)))
      (Variables|Default|SetSausageReffer _asbp_sausage))))

(event Collision|EventActorBeginOverlap
  (params (OtherActor :type Actor%20Object%20Reference))
  (CallFunction|DoDmg))

(event Collision|EventActorEndOverlap
  (params (OtherActor :type Actor%20Object%20Reference))
  (CallFunction|StopDmg))

(event EventDoDmg
  (bind _sausagereffer (Variables|Default|GetSausageReffer))
  (Variables|/Game/Character/BP_sausage.BP_sausage_C|Setisonfloor _sausagereffer true)
  (if (not (Variables|/Game/Character/BP_sausage.BP_sausage_C|GetisHot _sausagereffer))
    (Variables|/Game/Character/BP_sausage.BP_sausage_C|Setdamage (Variables|Default|GetSausageReffer) 2.0)
    (Default|ShowDMGMsg (Variables|Default|GetSausageReffer))
    (Utilities|FlowControl|Delay 5.0)
    (if (Variables|/Game/Character/BP_sausage.BP_sausage_C|Getisonfloor (Variables|Default|GetSausageReffer))
      (Variables|/Game/Character/BP_sausage.BP_sausage_C|Setdamage (Variables|Default|GetSausageReffer) 1e+01)
      (Default|ShowMoreDMGMSG (Variables|Default|GetSausageReffer)))))

(event EventStopDmg
  (bind _sausagereffer (Variables|Default|GetSausageReffer))
  (Variables|/Game/Character/BP_sausage.BP_sausage_C|Setisonfloor (Variables|Default|GetSausageReffer) false)
  (Variables|/Game/Character/BP_sausage.BP_sausage_C|Setdamage _sausagereffer 1.0)
  (Default|HideDMGMSG _sausagereffer))

(fn ConstructionScript)